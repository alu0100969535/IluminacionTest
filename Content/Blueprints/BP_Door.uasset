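; BP_Door is a door actor that swings between closed and open rotations when EventOpenClose fires.
; BeginPlay caches both end rotations and configures two opposing RotatingMovement components with mirrored rates and pivot offsets.
; EventOpenClose activates the component matching the current end rotation, ignoring calls at any other rotation.
; Tick times the swing, then deactivates the active component and snaps the root to the exact end rotation.
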(event Custom|EventOpenClose
  (bind _isclosed (CallFunction|DetectDoorClosed))
  (if _isclosed
    (Components|Activation|Activate (Variables|Default|GetPositiveRotatingMovement) false)
    (Variables|Default|SetCurrentOperationTime 0.0 :!label _label)
    (else
      (bind _isopen (CallFunction|DetectDoorOpen))
      (if _isopen
        (Components|Activation|Activate (Variables|Default|GetNegativeRotatingMovement) false)
        (goto _label)))))

(event EventBeginPlay
  (bind _pivotdisplacement (Variables|Default|GetPivotDisplacement))
  (bind _output_get (Variables|Default|SetInitialRotation (Transformation|GetWorldRotation (Variables|Default|GetDefaultSceneRoot))))
  (Variables|Default|SetFinalRotation (Math|Rotator|CombineRotators _output_get (Variables|Default|GetDeltaRotation)))
  (Variables|/Script/Engine.RotatingMovementComponent|SetRotationRate (Variables|Default|GetPositiveRotatingMovement) (Variables|Default|GetRotationRate))
  (Variables|/Script/Engine.RotatingMovementComponent|SetRotationRate (Variables|Default|GetNegativeRotatingMovement) (Class|KismetMathLibrary|NegateRotator (Variables|Default|GetRotationRate)))
  (Variables|/Script/Engine.RotatingMovementComponent|SetPivotTranslation (Variables|Default|GetPositiveRotatingMovement) _pivotdisplacement)
  (Variables|/Script/Engine.RotatingMovementComponent|SetPivotTranslation (Variables|Default|GetNegativeRotatingMovement) (* _pivotdisplacement -1.0)))

(event Collision|EventActorBeginOverlap
  (params (OtherActor :type Actor%20Object%20Reference)))

(event EventTick
  (params (DeltaSeconds :type Float%20%28single-precision%29))
  (bind _positiverotatingmovement (Variables|Default|GetPositiveRotatingMovement))
  (bind _negativerotatingmovement (Variables|Default|GetNegativeRotatingMovement))
  (bind _output_get (Variables|Default|SetCurrentOperationTime (+ DeltaSeconds (Variables|Default|GetCurrentOperationTime))))
  (if (> _output_get (Variables|Default|GetOperationTime))
    (if (Components|Activation|IsActive _positiverotatingmovement)
      (Components|Activation|Deactivate _positiverotatingmovement)
      (Transformation|SetWorldRotation (Variables|Default|GetDefaultSceneRoot) (Variables|Default|GetFinalRotation) false false)
      (Variables|Default|SetCurrentOperationTime 0.0 :!label _label)
      (elif (Components|Activation|IsActive _negativerotatingmovement)
        (Components|Activation|Deactivate _negativerotatingmovement)
        (Transformation|SetWorldRotation (Variables|Default|GetDefaultSceneRoot) (Variables|Default|GetInitialRotation) false false)
        (goto _label)))))

(fn ConstructionScript)

(fn DetectDoorClosed
  (return (Math|Rotator|Equal(Rotator) (Transformation|GetWorldRotation (Variables|Default|GetDefaultSceneRoot)) (Variables|Default|GetInitialRotation) 0.0001)))

(fn DetectDoorOpen
  (return (Math|Rotator|Equal(Rotator) (Transformation|GetWorldRotation (Variables|Default|GetDefaultSceneRoot)) (Variables|Default|GetFinalRotation) 0.0001)))